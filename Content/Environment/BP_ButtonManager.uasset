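; BP_ButtonManager handles presses of letter buttons in a letter-guessing game and reports whether each guess succeeds.
; It caches BP_GameModeBase on BeginPlay and extends the parent's OnButtonInteraction event.
; For an interactable HM_Button, it passes the letter to the game mode's TryRevealLetter and sets the button's press result from the returned value.
; A 2D success or failure sound plays accordingly, with non-interactable buttons also triggering the failure sound.
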(event `self.ReceiveBeginPlay`
  (bind _asbp_game_mode_base (cast `/Game/GameModes/BP_GameModeBase` (`GameplayStatics.GetGameMode`)))
  (set `self.BaseGameMode` _asbp_game_mode_base))

(event `self.OnButtonInteraction`
  (params (ButtonActor :type "HM_InteractiveActor Object Reference") (OtherActor :type "Actor Object Reference") (bCanBeInteractedWith :type Boolean))
  (bind _interactfailedsound (`self.InteractFailedSound`))
  (bind _interactsuccesssound (`self.InteractSuccessSound`))
  (bind _interactfailedsound_2 (`self.InteractFailedSound`))
  (`parent.OnButtonInteraction` ButtonActor OtherActor bCanBeInteractedWith)
  (`/Engine/EditorBlueprintResources/StandardMacros.IsValid` (`self.BaseGameMode`)
    (:`Is Valid`
      (if bCanBeInteractedWith
        (bind _ashm_button (cast `HM_Button` ButtonActor))
        (bind _returnvalue (`HM_GameModeBase.TryRevealLetter` (`self.BaseGameMode`) (`KismetTextLibrary.Conv_TextToString` (`HM_Button.K2_GetLetter` _ashm_button))))
        (bind _returnvalue_2 (> _returnvalue 0))
        (`HM_Button.SetPressResult` _ashm_button _returnvalue_2)
        (if _returnvalue_2
          (`/Engine/EditorBlueprintResources/StandardMacros.IsValid` _interactsuccesssound
            (:`Is Valid`
              (`GameplayStatics.PlaySound2D` _interactsuccesssound 1.0 1.0 0.0 null null)))
          (else
            (`/Engine/EditorBlueprintResources/StandardMacros.IsValid` _interactfailedsound
              (:`Is Valid`
                (`GameplayStatics.PlaySound2D` _interactfailedsound 1.0 1.0 0.0 null null)))))
        (else
          (`/Engine/EditorBlueprintResources/StandardMacros.IsValid` _interactfailedsound_2
            (:`Is Valid`
              (`GameplayStatics.PlaySound2D` _interactfailedsound_2 1.0 1.0 0.0 null null))))))))

(fn `UserConstructionScript`)