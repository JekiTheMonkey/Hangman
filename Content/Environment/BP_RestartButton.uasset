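; An interactable restart button that calls Restart on BP_GameModeBase and changes its look with the game state.
; On BeginPlay it caches the button's default material and the text's, then binds to the game mode's game-over and restart delegates.
; Game over applies a win or lose material to the button; the matching text material change is disconnected and never runs.
; Restart restores both default materials.
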(event `self.ReceiveBeginPlay`
  (set `self.DefaultButtonMaterial` (`PrimitiveComponent.GetMaterial` (`self.RestatButton`) 0))
  (set `self.DefaultFontMaterial` (`PrimitiveComponent.GetMaterial` (`self.RestartText`) 0))
  (bind _asbp_game_mode_base (cast `/Game/GameModes/BP_GameModeBase` (`GameplayStatics.GetGameMode`)))
  (bind _output_get (set `self.GameModeBase` _asbp_game_mode_base))
  (add `HM_GameModeBase.GameOverDelegate` _output_get (`|CreateDelegate` :!event `OnGameOver`))
  (add `HM_GameModeBase.RestartDelegate` _output_get (`|CreateDelegate` :!event `OnRestart`)))

(event `self.Interact`
  (params (OtherActor :type "Actor Object Reference"))
  (bind _gamemodebase (`self.GameModeBase`))
  (`/Engine/EditorBlueprintResources/StandardMacros.IsValid` _gamemodebase
    (:`Is Valid`
      (`/Game/GameModes/BP_GameModeBase.Restart` _gamemodebase))))

(fn `OnGameOver`
  (params (bSuccess :type Boolean))
  (bind _returnvalue (select `bool` (`local.bSuccess`) :`false` (`self.GameLoseButtonMaterial`) :`true` (`self.GameWinButtonMaterial`)))
  (`|ExecutionSequence`
    (:`then_1`
      ;[1 1 1] Set button material.
      (`/Engine/EditorBlueprintResources/StandardMacros.IsValid` _returnvalue
        (:`Is Valid`
          (`PrimitiveComponent.SetMaterial` (`self.RestatButton`) 0 _returnvalue))))))

(fn `OnRestart`
  (bind _defaultfontmaterial (`self.DefaultFontMaterial`))
  (bind _defaultbuttonmaterial (`self.DefaultButtonMaterial`))
  (`|ExecutionSequence`
    (:`then_0`
      (`/Engine/EditorBlueprintResources/StandardMacros.IsValid` _defaultfontmaterial
        (:`Is Valid`
          (`TextRenderComponent.SetTextMaterial` (`self.RestartText`) _defaultfontmaterial))))
    (:`then_1`
      (`/Engine/EditorBlueprintResources/StandardMacros.IsValid` _defaultbuttonmaterial
        (:`Is Valid`
          (`PrimitiveComponent.SetMaterial` (`self.RestatButton`) 0 _defaultbuttonmaterial))))))

(fn `UserConstructionScript`)