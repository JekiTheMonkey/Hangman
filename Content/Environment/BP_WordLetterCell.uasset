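; BP_WordLetterCell is a letter cell actor that flips over to reveal the letter on its back.
; On BeginPlay the letter text is hidden unless Debug is set.
; Reveal shows the text and starts a looping timer that pitches the actor in steps, plus a one-shot timer to end the flip.
; EndReveal stops the loop and snaps to exactly 180 degrees from the original rotation to remove float drift.
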(event `self.ReceiveBeginPlay`
  ;[1 1 1] The letter is on back.
  (`SceneComponent.SetHiddenInGame` (`self.LetterTextRender`) (not (`self.bDebug`)) false))

(event `self.Reveal`
  (`SceneComponent.SetHiddenInGame` (`self.LetterTextRender`) false false)
  (set `self.OriginalRotation` (`self.K2_GetActorRotation`))
  (bind _returnvalue (`KismetSystemLibrary.K2_SetTimerDelegate` (delegate `RevealTick`) (/ (`self.SecondsToReveal`) (`self.RevealTickRate`)) true))
  (`KismetSystemLibrary.K2_SetTimerDelegate` (delegate `EndReveal`) (`self.SecondsToReveal`)))

(event `RevealTick`
  (`self.K2_AddActorLocalRotation` (`KismetMathLibrary.MakeRotator` 0.0 (/ 180.0 (* (`self.RevealTickRate`) (`self.SecondsToReveal`))))))

(event `EndReveal`
  (`KismetSystemLibrary.K2_ClearAndInvalidateTimerHandle` (stale `self.Reveal` _returnvalue))
  ;[1 1 1] Fix floating point imprecisions.
  (`self.K2_SetActorRotation` (`self.OriginalRotation`) true)
  (`self.K2_AddActorLocalRotation` (struct :`Pitch` 180.0) false true))

(fn `UserConstructionScript`)