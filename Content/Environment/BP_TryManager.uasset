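; BP_TryManager is a placed actor that shows the player's failed tries as a row of BP_TryCell actors.
; On BeginPlay it spawns one cell per MaxTries from BP_MainGame_GM, offset from its own transform by DistanceBetween, and binds to the game mode's restart and try-failed delegates.
; Each failure sets the next cell's status to true and advances TryIndex, while a restart resets the index and every cell.
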(event `self.ReceiveBeginPlay`
  (bind _asbp_main_game_gm (cast `/Game/GameModes/BP_MainGame_GM` (`GameplayStatics.GetGameMode`)))
  (for _index (range 1 (+ (`HM_GameModeBase.MaxTries` _asbp_main_game_gm) 1))
    (bind _returnvalue (`|SpawnActorFromClass` "/Game/Environment/BP_TryCell.BP_TryCell_C" (`KismetMathLibrary.MakeTransform` (+ (`self.K2_GetActorLocation`) (* (`self.DistanceBetween`) (- _index 1))) (`self.K2_GetActorRotation`) (`self.GetActorScale3D`)) "AlwaysSpawn" "OverrideRootScale" null null))
    (`KismetArrayLibrary.Array_Add` (`self.Tries`) _returnvalue))
  (add `HM_GameModeBase.RestartDelegate` _asbp_main_game_gm (`|CreateDelegate` :!event `OnRestart`))
  (add `HM_GameModeBase.OnTryFailedDelegate` _asbp_main_game_gm (`|CreateDelegate` :!event `OnTryFailed`)))

(fn `OnRestart`
  (set `self.TryIndex` 0)
  (for _array_element (`self.Tries`)
    (`/Game/Environment/BP_TryCell.SetStatus` _array_element false)))

(fn `OnTryFailed`
  (bind _output (`|GetArrayItem` (`self.Tries`) (`self.TryIndex`)))
  (`/Engine/EditorBlueprintResources/StandardMacros.IsValid` _output
    (:`Is Valid`
      (`/Game/Environment/BP_TryCell.SetStatus` _output true)
      (`/Engine/EditorBlueprintResources/StandardMacros.IncrementInt` (`self.TryIndex`)))))

(fn `UserConstructionScript`)