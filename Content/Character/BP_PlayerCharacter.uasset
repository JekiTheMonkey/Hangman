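; Player character Blueprint that lets the player target tagged objects with an Interact input.
; On press, it line traces forward from the camera on the Visibility channel over a configurable length, with optional persistent debug drawing.
; A hit actor tagged "Interact" is passed to the Interact function, which currently only prints that actor's display name.
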(event `InputAction|Interact`
  (params (Key :type "Key Structure"))
  (bind _camera (`self.Camera`))
  (bind _returnvalue (`SceneComponent.K2_GetComponentLocation` _camera))
  (:`Pressed`
    (bind (_outhit _returnvalue_2) (`KismetSystemLibrary.LineTraceSingle` :`Start` _returnvalue :`End` (+ _returnvalue (* (`SceneComponent.GetForwardVector` _camera) (`self.InteractTraceLength`))) :`TraceChannel` "TraceTypeQuery1" :`DrawDebugType` (select `bool` (`self.bDebugInteractTrace`) :`true` "Persistent" :!type "EDrawDebugTrace Enum")))
    (if _returnvalue_2
      (bind (_bblockinghit _binitialoverlap _time _distance _location _impactpoint _normal _impactnormal _physmat _hitactor) (`GameplayStatics.BreakHitResult` _outhit))
      (if (`self.ActorHasTag` _hitactor "Interact")
        (`self.Interact` _hitactor)))))

(fn `Interact`
  (params (Object :type "Actor Object Reference"))
  (`KismetSystemLibrary.PrintString` (`KismetSystemLibrary.GetDisplayName` Object)))

(fn `UserConstructionScript`)